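; Base Blueprint for interactive prop objects, carrying debug hooks for puzzle events.
; A debug graph prints the object's name with the event when a puzzle activates, and shows a longer-lasting orange warning when an event is invalid or unassigned.
; BeginPlay and the construction script are empty, and nothing in these graphs calls the debug events.
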(event `self.ReceiveBeginPlay`)

(event `Debug_PuzzleActivated`
  (params (EventToActivate :type Name))
  (`KismetSystemLibrary.PrintString` (`KismetStringLibrary.Concat_StrStr` (`KismetSystemLibrary.GetObjectName` self) "::" (`KismetStringLibrary.Conv_NameToString` EventToActivate) "::" "Puzzle Activated")))

(event `Debug_PuzzleInvalid`
  (params (EventUnassigned :type Name))
  (`KismetSystemLibrary.PrintString` (`KismetStringLibrary.Concat_StrStr` (`KismetSystemLibrary.GetObjectName` self) "" (`KismetStringLibrary.Conv_NameToString` EventUnassigned) "" "Event NOT VALID!!") true true (struct :`R` 1.0 :`G` 0.488864 :`A` 1.0) 5.0))

(fn `UserConstructionScript`)