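; Base Blueprint for interactive restore-target props, which track player proximity for a put-back slots manager.
; Overlap begin and end on the PlayerDetectionZone forward the other actor to CYPutBackSlotsManagerComp as detection enter and exit.
; Puzzle-state events switch on initial state and event name, but only as stubs: no case logic is shown beyond a debug print in the event-call handler.
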(event `self.PlayerDetectionZone.OnComponentBeginOverlap`
  (params (OverlappedComponent :type "PrimitiveComponent Object Reference") (OtherActor :type "Actor Object Reference") (OtherComp :type "PrimitiveComponent Object Reference") (OtherBodyIndex :type Integer) (bFromSweep :type Boolean) (SweepResult :type "HitResult Structure (by ref)"))
  (`/Game/UActors/CY_Props/RestoreTargets/PutBackTarget/CY_PutBackSlotsManager_Comp.Player Enter Detection` (`self.CY_PutBackSlotsManager_Comp`) OtherActor))

(event `self.PlayerDetectionZone.OnComponentEndOverlap`
  (params (OverlappedComponent :type "PrimitiveComponent Object Reference") (OtherActor :type "Actor Object Reference") (OtherComp :type "PrimitiveComponent Object Reference") (OtherBodyIndex :type Integer))
  (`/Game/UActors/CY_Props/RestoreTargets/PutBackTarget/CY_PutBackSlotsManager_Comp.Player Exit Detection` (`self.CY_PutBackSlotsManager_Comp`) OtherActor))

(event `self.CY_Widgets_PuzzleStatesEvents.OnIntializePropState`
  (params (InitialState :type "/Game/UComponents/Util/CY_EPropStates_Enum Enum" :default "NewEnumerator4"))
  (switch `/Game/UComponents/Util/CY_EPropStates_Enum` InitialState))

(event `self.CY_Widgets_PuzzleStatesEvents.OnPropPuzzleEventCall`
  (params (EventName :type Name))
  (switch `name` EventName
    (:`DebugCall`
      (`KismetSystemLibrary.PrintString` "EventCallPassed::PutBackEvent" true true (struct :`R` 1.0 :`G` 0.557167 :`A` 1.0) 10.0))))

(fn `UserConstructionScript`
  (`parent.UserConstructionScript`))