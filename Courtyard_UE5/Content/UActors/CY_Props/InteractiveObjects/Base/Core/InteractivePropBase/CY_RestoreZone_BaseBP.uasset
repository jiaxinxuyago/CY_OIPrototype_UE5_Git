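; Base Blueprint for a restore zone prop that detects overlapping actors for a put-back slots manager component.
; Begin and end overlaps on its player detection zone are forwarded to the manager as player enter and exit calls.
; Debug events print puzzle activation messages and orange warnings for invalid events, tagged with the object or event name.
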(event `self.ReceiveBeginPlay`)

(event `self.PlayerDetectionZone.OnComponentBeginOverlap`
  (params (OverlappedComponent :type "PrimitiveComponent Object Reference") (OtherActor :type "Actor Object Reference") (OtherComp :type "PrimitiveComponent Object Reference") (OtherBodyIndex :type Integer) (bFromSweep :type Boolean) (SweepResult :type "HitResult Structure (by ref)"))
  (`/Game/UActors/CY_Props/RestoreTargets/PutBackTarget/CY_PutBackSlotsManager_Comp.Player Enter Detection` (`self.CY_PutBackSlotsManager_Comp`) OtherActor))

(event `self.PlayerDetectionZone.OnComponentEndOverlap`
  (params (OverlappedComponent :type "PrimitiveComponent Object Reference") (OtherActor :type "Actor Object Reference") (OtherComp :type "PrimitiveComponent Object Reference") (OtherBodyIndex :type Integer))
  (`/Game/UActors/CY_Props/RestoreTargets/PutBackTarget/CY_PutBackSlotsManager_Comp.Player Exit Detection` (`self.CY_PutBackSlotsManager_Comp`) OtherActor))

(event `Debug_PuzzleActivated`
  (params (EventToActivate :type Name))
  (`KismetSystemLibrary.PrintString` (`KismetStringLibrary.Concat_StrStr` (`KismetSystemLibrary.GetObjectName` self) "::" (`KismetStringLibrary.Conv_NameToString` EventToActivate) "::" "Puzzle Activated")))

(event `Debug_PuzzleInvalid`
  (params (EventUnassigned :type Name))
  (`KismetSystemLibrary.PrintString` (`KismetStringLibrary.Concat_StrStr` (`KismetSystemLibrary.GetObjectName` self) "" (`KismetStringLibrary.Conv_NameToString` EventUnassigned) "" "Event NOT VALID!!") true true (struct :`R` 1.0 :`G` 0.488864 :`A` 1.0) 5.0))

(fn `UserConstructionScript`)