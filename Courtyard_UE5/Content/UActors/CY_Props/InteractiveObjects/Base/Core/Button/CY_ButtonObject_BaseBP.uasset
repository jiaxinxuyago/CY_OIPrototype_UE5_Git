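; Base Blueprint for interactive button props, tagged with its interactive class type in the construction script.
; A detection zone forwards begin and end overlaps to the button handler component as player enter and exit notifications.
; When the handler component fires its button behavior event, the actor plays its ActorSequence as the press response.
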(event `self.CY_ButtonHandler_Comp.ButtonBehavior`
  (`MovieSceneSequencePlayer.Play` (`ActorSequenceComponent.SequencePlayer` (`self.ActorSequence`))))

(event `self.PlayerDetectionZone.OnComponentBeginOverlap`
  (params (OverlappedComponent :type "PrimitiveComponent Object Reference") (OtherActor :type "Actor Object Reference") (OtherComp :type "PrimitiveComponent Object Reference") (OtherBodyIndex :type Integer) (bFromSweep :type Boolean) (SweepResult :type "HitResult Structure (by ref)"))
  (`/Game/UActors/CY_Props/InteractiveObjects/Base/Core/Button/CY_ButtonHandler_Comp.PlayerEnterDetection` (`self.CY_ButtonHandler_Comp`) OtherActor))

(event `self.PlayerDetectionZone.OnComponentEndOverlap`
  (params (OverlappedComponent :type "PrimitiveComponent Object Reference") (OtherActor :type "Actor Object Reference") (OtherComp :type "PrimitiveComponent Object Reference") (OtherBodyIndex :type Integer))
  (`/Game/UActors/CY_Props/InteractiveObjects/Base/Core/Button/CY_ButtonHandler_Comp.PlayerExitDetection` (`self.CY_ButtonHandler_Comp`) OtherActor))

(fn `UserConstructionScript`
  (`parent.UserConstructionScript`)
  (set `self.EInteractiveClassType` "NewEnumerator6"))