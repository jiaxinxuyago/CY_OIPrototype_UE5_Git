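; Base trigger volume Blueprint that raises CY event-link enter and exit events when the main character overlaps it.
; Begin and end overlaps are filtered by a cast to CY_Main_CharacterBP, so other actors are ignored.
; The puzzle states component switches the volume on or off, through its initial state and puzzle events, by toggling collision between query-only and disabled.
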(event `self.ReceiveActorBeginOverlap`
  (params (OtherActor :type "Actor Object Reference"))
  (cast `/Game/UActors/CY_Characters/MainCharacter/CY_Main_CharacterBP` OtherActor)
  (`/Game/UComponents/Util/CY_ObjectInteraction_FunctionLibrary.CY Event Link on Trigger Enter` self))

(event `self.ReceiveActorEndOverlap`
  (params (OtherActor :type "Actor Object Reference"))
  (cast `/Game/UActors/CY_Characters/MainCharacter/CY_Main_CharacterBP` OtherActor)
  (`/Game/UComponents/Util/CY_ObjectInteraction_FunctionLibrary.CY Event Link on Trigger Exit` self))

(event `self.CY_PuzzleStatesEvents_Comp.OnIntializePropState`
  (params (InitialState :type "/Game/UComponents/Util/CY_EPropStates_Enum Enum" :default "NewEnumerator4"))
  (switch `/Game/UComponents/Util/CY_EPropStates_Enum` InitialState
    (:`NewEnumerator0`
      (`self.TurnOnTriggerVol`))
    (:`NewEnumerator5`
      (`self.TurnOffTriggerVol`))))

(event `self.CY_PuzzleStatesEvents_Comp.OnPropPuzzleEventCall`
  (params (EventName :type Name))
  (switch `name` EventName
    (:`TurnOn`
      (`self.TurnOnTriggerVol`))
    (:`TurnOff`
      (`self.TurnOffTriggerVol`))))

(fn `TurnOffTriggerVol`
  (`PrimitiveComponent.SetCollisionEnabled` (`self.CollisionComponent`) "NoCollision"))

(fn `TurnOnTriggerVol`
  (`PrimitiveComponent.SetCollisionEnabled` (`self.CollisionComponent`) "QueryOnly"))

(fn `UserConstructionScript`)