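; Base Blueprint for consumable interactive props, handling what happens when the object is consumed.
; The construction script runs the parent's, then tags the actor with an interactive class type enum value.
; The Consuming event spawns an enlarged sparks effect at the actor's location, then after a short delay destroys both the effect and the actor.
; BeginPlay, overlap and Tick are disabled stubs.
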(event `Consuming`
  (bind _returnvalue (`GameplayStatics.SpawnEmitterAtLocation` "/Game/3CTemplates/StarterContent/Particles/P_Sparks.P_Sparks" (`self.K2_GetActorLocation`) (struct) (5.0 5.0 5.0)))
  (`KismetSystemLibrary.Delay` 0.3)
  (`ActorComponent.K2_DestroyComponent` _returnvalue)
  (`self.K2_DestroyActor`))

(fn `UserConstructionScript`
  (`parent.UserConstructionScript`)
  (set `self.EInteractiveClassType` "NewEnumerator1"))