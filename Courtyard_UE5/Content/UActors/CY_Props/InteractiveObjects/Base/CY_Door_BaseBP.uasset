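; Base Blueprint for an interactive door prop that puzzle events open and close.
; It listens to puzzle-state events, snapping the door to its initial pose or handling Open and Close calls by name.
; Opening and closing check an IsOpen flag, play the matching level sequence, then immediately set the door's relative rotation.
; The initial-state snap only sets rotation and leaves IsOpen untouched.
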(event `self.CY_Widgets_PuzzleStatesEvents.OnIntializePropState`
  (params (InitialState :type "/Game/UComponents/Util/CY_EPropStates_Enum Enum" :default "NewEnumerator4"))
  (switch `/Game/UComponents/Util/CY_EPropStates_Enum` InitialState
    (:`NewEnumerator6`
      (`self.SnapToOpen`))
    (:`NewEnumerator7`
      (`self.SnapToClose`))))

(event `self.CY_Widgets_PuzzleStatesEvents.OnPropPuzzleEventCall`
  (params (EventName :type Name))
  (switch `name` EventName
    (:`Open`
      (`self.OpenDoor`))
    (:`Close`
      (`self.CloseDoor`))))

(fn `CloseDoor`
  (if (`self.IsOpen`)
    (`MovieSceneSequencePlayer.Play` (`ActorSequenceComponent.SequencePlayer` (`self.DoorCloseSequence`)))
    (set `self.IsOpen` false)
    (`self.SnapToClose`)))

(fn `OpenDoor`
  (if (not (`self.IsOpen`))
    (`MovieSceneSequencePlayer.Play` (`ActorSequenceComponent.SequencePlayer` (`self.DoorOpenSequence`)))
    (set `self.IsOpen` true)
    (`self.SnapToOpen`)))

(fn `SnapToClose`
  (`SceneComponent.K2_SetRelativeRotation` :`self` (`self.Door`)))

(fn `SnapToOpen`
  (`SceneComponent.K2_SetRelativeRotation` (`self.Door`) (struct :`Yaw` -90.0) false false))

(fn `UserConstructionScript`
  (`parent.UserConstructionScript`))