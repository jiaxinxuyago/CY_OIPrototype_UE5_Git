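; A test interactive cup prop that swaps its material in response to puzzle state events.
; Initial state, named puzzle events and integer state toggles all route to Set Black, Set White or Set Gold, each replacing the mesh's first material slot.
; The construction script sets the interactive class type and calls the tag setup for the put-back and grab components.
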(event `self.ReceiveBeginPlay`
  (`parent.ReceiveBeginPlay`))

(event `self.ReceiveTick`
  (params (DeltaSeconds :type "Float (single-precision)"))
  (`parent.ReceiveTick` DeltaSeconds))

(event `self.CY_Widgets_PuzzleStatesEvents.OnIntializePropState`
  (params (InitialState :type "/Game/UComponents/Util/CY_EPropStates_Enum Enum" :default "NewEnumerator4"))
  (switch `/Game/UComponents/Util/CY_EPropStates_Enum` InitialState
    (:`NewEnumerator0`
      (`self.Set Black`))
    (:`NewEnumerator5`
      (`self.SetGold`))))

(event `self.CY_Widgets_PuzzleStatesEvents.OnPropPuzzleEventCall`
  (params (EventName :type Name))
  (switch `name` EventName
    (:`setBlack`
      (`self.Set Black`))
    (:`SetWhite`
      (`self.Set White`))
    (:`SetGold`
      (`self.SetGold`))))

(event `self.CY_Widgets_PuzzleStatesEvents.OnPropPuzzleStateToggle`
  (params (StateInt :type Integer))
  (switch `int` StateInt
    (:`0`
      (`self.Set Black`))
    (:`1`
      (`self.Set White`))
    (:`2`
      (`self.SetGold`))))

(fn `Set Black`
  (`PrimitiveComponent.SetMaterial` (`self.Object`) 0 "/Game/3CTemplates/TPSAT/Materials/Objects/M_Mug.M_Mug"))

(fn `Set White`
  (`PrimitiveComponent.SetMaterial` (`self.Object`) 0 "/Game/3CTemplates/TPSAT/Materials/Environment/M_WhiteBox.M_WhiteBox"))

(fn `SetGold`
  (`PrimitiveComponent.SetMaterial` (`self.Object`) 0 "/Game/3CTemplates/StarterContent/Materials/M_Metal_Gold.M_Metal_Gold"))

(fn `UserConstructionScript`
  (`parent.UserConstructionScript`)
  (set `self.EInteractiveClassType` "NewEnumerator0")
  (`/Game/UComponents/Util/CY_ObjectInteraction_FunctionLibrary.CY Set Tag on Put Back Comp` null)
  (`/Game/UComponents/Util/CY_ObjectInteraction_FunctionLibrary.CY Set Tag on Grab Comp` null))