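; Base puzzle manager Blueprint that detects when a set of puzzle pieces is solved and plays a level sequence.
; Each Tick adds every piece's CY_PropLink_Comp score to a running total, never reset between frames, and compares it to the piece count.
; A match fires the solved events once, starting PuzzleLevelSeq.
; The loop over PuzzlePropsToActivate is empty, with its CallPuzzleEvent node left unconnected.
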(event `self.ReceiveBeginPlay`
  (set `self.FullPuzzleScore` (`KismetArrayLibrary.Array_Length` (`self.PuzzlePieces`)))
  (set `self.CurrentPuzzleScore` 0))

(event `self.ReceiveTick`
  (params (DeltaSeconds :type "Float (single-precision)"))
  (`|ExecutionSequence`
    (:`then_0`
      (for _array_element (`self.PuzzlePieces`)
        (bind _returnvalue (`self.GetComponentByClass` _array_element "/Game/UComponents/Components/CY_PropLink_Comp.CY_PropLink_Comp_C"))
        (`/Engine/EditorBlueprintResources/StandardMacros.IsValid` _returnvalue
          (:`Is Valid`
            (set `self.CurrentPuzzleScore` (+ (`/Game/UComponents/Components/CY_PropLink_Comp.PuzzlePieceScore` _returnvalue) (`self.CurrentPuzzleScore`)))))))
    (:`then_1`
      (if (== (`self.CurrentPuzzleScore`) (`self.FullPuzzleScore`))
        (`/Engine/EditorBlueprintResources/StandardMacros.DoOnce` false
          (:`Completed`
            (`self.OnPuzzleSolved`)
            (`self.OnPuzzleSeqSolved`)))))))

(event `OnPuzzleSolved`
  (for _ (`self.PuzzlePropsToActivate`)
    _))

(event `OnPuzzleSeqSolved`
  (bind (_outactor _returnvalue) (`LevelSequencePlayer.CreateLevelSequencePlayer` (`self.PuzzleLevelSeq`)))
  (`MovieSceneSequencePlayer.Play` _returnvalue))

(fn `UserConstructionScript`)