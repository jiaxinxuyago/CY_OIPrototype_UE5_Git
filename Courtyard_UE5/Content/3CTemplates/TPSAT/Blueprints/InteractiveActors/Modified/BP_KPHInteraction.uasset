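; Interactive actor that runs a one-shot, timed media and lighting sequence through its TopButtonInteraction event.
; The event opens a source on a second media player and reveals a plane, then after a short delay opens the main player and sets red, green and blue spotlight intensities.
; Further delays destroy the plane, then the three spotlights, with no reset logic.
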(event `/Game/3CTemplates/TPSAT/Blueprints/Core/BaseActors/BP_Base_InteractiveObject.TopButtonInteraction`
  (`MediaPlayer.OpenSource` (`self.MediaPlayer2`) null)
  (`SceneComponent.SetVisibility` (`StaticMeshActor.StaticMeshComponent` (`self.Plane1`)) true false)
  (`KismetSystemLibrary.Delay` 2.0)
  (`MediaPlayer.OpenSource` (`self.MediaPlayer`) null)
  (`LightComponent.SetIntensity` (`Light.LightComponent` (`self.SpotlightR`)) 160.0)
  (`LightComponent.SetIntensity` (`Light.LightComponent` (`self.SpotlightG`)) 160.0)
  (`LightComponent.SetIntensity` (`Light.LightComponent` (`self.SpotlightB`)) 160.0)
  (`KismetSystemLibrary.Delay` 3.0)
  (`self.K2_DestroyActor` (`self.Plane1`))
  (`KismetSystemLibrary.Delay` 8.0)
  (`self.K2_DestroyActor` (`self.SpotlightR`))
  (`self.K2_DestroyActor` (`self.SpotlightG`))
  (`self.K2_DestroyActor` (`self.SpotlightB`)))

(fn `UserConstructionScript`
  (`parent.UserConstructionScript`))