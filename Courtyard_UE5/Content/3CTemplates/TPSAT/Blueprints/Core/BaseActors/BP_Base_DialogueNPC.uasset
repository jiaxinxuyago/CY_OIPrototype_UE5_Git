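; Base NPC actor for branching, cinematic conversations, with a top-button player comment and a bottom-button talk.
; Talking hides player, NPC and widgets, then chains data table rows as either NPC lines or player choices over a looping Level Sequence.
; Chosen options play their sequence and can spawn consequence scripts, while timers show subtitles timed by text length.
; Finished conversations are saved to the game instance, leaving an optional follow-up comment.
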(event `/Game/3CTemplates/TPSAT/Blueprints/Core/BP_InteractionInterface.Interaction`
  (params (GameController :type "/Game/3CTemplates/TPSAT/Blueprints/Core/BP_StoryAdv_GameController Object Reference") (Button :type "/Game/3CTemplates/TPSAT/Blueprints/Core/Enums/EInteractionButtons Enum" :default "NewEnumerator0"))
  ;[0 0.7379 1] Handle interaction event
  (set `self.GameControllerInstance` GameController)
  (switch `/Game/3CTemplates/TPSAT/Blueprints/Core/Enums/EInteractionButtons` Button
    (:`NewEnumerator0`
      ;;[1 1 1] Focus on and play comment as dialogue
      (`|ExecutionSequence`
        (:`then_0`
          (bind (_dialogue_waves _subtitles _validdata) (`/Game/3CTemplates/TPSAT/Blueprints/Core/BP_StoryAdv_FunctionLibrary.GetDialogueDataFromTable` (`self.DialogueRow`)))
          (if _validdata
            (`/Game/3CTemplates/TPSAT/Blueprints/Core/BP_StoryAdv_GameController.PlayPlayerDialogue` (`self.GameControllerInstance`) _dialogue_waves _subtitles)))
        (:`then_1`
          (if (`self.UseCameraFocus`)
            (`self.CameraFocus`)))))
    (:`NewEnumerator1`
      (if (`self.ConversationOver`)
        (`self.PlayCommentSequence`)
        (else
          (`self.PrepareConversation`))))))

(event `PrepareConversation`
  ;[0 0.7379 1] Prepare for conversation
  (set `self.NextUp` (`self.StartingPoint`))
  (set `/Game/3CTemplates/TPSAT/Blueprints/Core/BP_StoryAdv_GameController.HoldTrace` true (`self.GameControllerInstance`))
  (bind _hiddenwidgets (`/Game/3CTemplates/TPSAT/Blueprints/Core/BP_StoryAdv_FunctionLibrary.HideActiveWidgets`))
  (set `self.HiddenWidgets` _hiddenwidgets)
  (`SceneComponent.SetHiddenInGame` (`self.Character`) true true)
  (`self.SetActorHiddenInGame` (`GameplayStatics.GetPlayerPawn` 0) true)
  (`self.DisableInput` (`self.GameControllerInstance`) (`GameplayStatics.GetPlayerController` 0))
  (`self.DisableInput` (`GameplayStatics.GetPlayerPawn` 0) (`GameplayStatics.GetPlayerController` 0))
  (`/Engine/EditorBlueprintResources/StandardMacros.IsValid` (`self.IntroSequence`)
    (:`Is Valid`
      (bind _outactor (`LevelSequencePlayer.CreateLevelSequencePlayer` (`self.IntroSequence`)))
      (bind _output_get (set `self.SequencePlayer` _outactor))
      (bind _sequenceplayer (`LevelSequenceActor.SequencePlayer` _output_get))
      (`MovieSceneSequencePlayer.Play` _sequenceplayer)
      (add `MovieSceneSequencePlayer.OnFinished` _sequenceplayer (delegate `CarryOnConversation`)))
    (:`Is Not Valid`
      (`self.CarryOnConversation`))))

(event `CarryOnConversation`
  ;[0 0.7379 1] Prepare for conversation
  (`self.NextDialogue` (`self.NextUp`)))

(event `DialogueOptions`
  (params (Options :type "Array of /Game/3CTemplates/TPSAT/Blueprints/Core/Structures/Conversation_PlayerOptions Structure") (LoopSequence :type "LevelSequence Object Reference"))
  (bind _dialoguewidget (`self.DialogueWidget`))
  ;[0 0.7379 1] Display dialogue options
  (set `self.CurrentDialogueOptions` Options)
  (`/Engine/EditorBlueprintResources/StandardMacros.IsValid` (`self.SequencePlayer`)
    (:`Is Valid`
      _)
    (:`Is Not Valid`
      (bind _outactor (`LevelSequencePlayer.CreateLevelSequencePlayer` LoopSequence))
      (set `self.SequencePlayer` _outactor)))
  (`LevelSequenceActor.SetSequence` (`self.SequencePlayer`) LoopSequence)
  (`MovieSceneSequencePlayer.PlayLooping` (`LevelSequenceActor.SequencePlayer` (`self.SequencePlayer`)) -1)
  (`/Engine/EditorBlueprintResources/StandardMacros.IsValid` (`self.DialogueWidget`)
    (:`Is Valid`
      _)
    (:`Is Not Valid`
      (bind _returnvalue (`|CreateWidget` "/Game/3CTemplates/TPSAT/UserInterface/WBP_DialogueOptions.WBP_DialogueOptions_C" null self))
      (set `self.DialogueWidget` _returnvalue)))
  (`UserWidget.AddToViewport` (`self.DialogueWidget`) 0)
  (set `/Game/3CTemplates/TPSAT/UserInterface/WBP_DialogueOptions.NumberOfChoices` (`KismetArrayLibrary.Array_Length` (`self.CurrentDialogueOptions`)) _dialoguewidget)
  (`/Game/3CTemplates/TPSAT/UserInterface/WBP_DialogueOptions.SetButtonVisibility` _dialoguewidget)
  (for (_array_element _array_index) (`self.CurrentDialogueOptions`)
    (`/Game/3CTemplates/TPSAT/UserInterface/WBP_DialogueOptions.SetUpOptions` (`self.DialogueWidget`) (`.Text_19_B110F5F04F1AF3B3C13A2C959DA3D719` (break `/Game/3CTemplates/TPSAT/Blueprints/Core/Structures/Conversation_PlayerOptions` _array_element)) _array_index)))

(fn `DisableTalkButton`
  (switch `/Game/3CTemplates/TPSAT/Blueprints/Core/Enums/EInteractionButtons` (`self.TalkButton`)
    (:`NewEnumerator0`
      (setmembers `/Game/3CTemplates/TPSAT/Blueprints/Core/Structures/BP_InteractionLabels` :`StructRef` (`self.InteractionButtons`) :`Top Button` ""))
    (:`NewEnumerator1`
      (setmembers `/Game/3CTemplates/TPSAT/Blueprints/Core/Structures/BP_InteractionLabels` :`StructRef` (`self.InteractionButtons`) :`Bottom Button` ""))
    (:`NewEnumerator2`
      (setmembers `/Game/3CTemplates/TPSAT/Blueprints/Core/Structures/BP_InteractionLabels` :`StructRef` (`self.InteractionButtons`) :`Left Button` ""))
    (:`NewEnumerator3`
      (setmembers `/Game/3CTemplates/TPSAT/Blueprints/Core/Structures/BP_InteractionLabels` :`StructRef` (`self.InteractionButtons`) :`Right Button` ""))))

(fn `EndConversation`
  (`/Game/3CTemplates/TPSAT/Blueprints/Core/BP_StoryAdv_FunctionLibrary.ShowHiddenWidgets` (`self.HiddenWidgets`))
  (set `/Game/3CTemplates/TPSAT/Blueprints/Core/BP_StoryAdv_GameController.HoldTrace` false (`self.GameControllerInstance`))
  (`SceneComponent.SetHiddenInGame` (`self.Character`) false true)
  (`self.SetActorHiddenInGame` (`GameplayStatics.GetPlayerPawn` 0) false)
  (`self.EnableInput` (`GameplayStatics.GetPlayerPawn` 0) (`GameplayStatics.GetPlayerController` 0))
  (`self.EnableInput` (`self.GameControllerInstance`) (`GameplayStatics.GetPlayerController` 0))
  (clear `MovieSceneSequencePlayer.OnFinished` (`LevelSequenceActor.SequencePlayer` (`self.SequencePlayer`)))
  ;[1 1 1] Remember this conversation status for saving and loading
  (`KismetArrayLibrary.Array_Add` (`/Game/3CTemplates/TPSAT/Blueprints/Core/BP_StoryAdv_GameInstance.FinishedConversations` (`/Game/3CTemplates/TPSAT/Blueprints/Core/BP_StoryAdv_FunctionLibrary.GetStoryAdvGameInstance`)) (`KismetSystemLibrary.GetObjectName` self))
  ;[1 1 1] Remove level sequence actor
  (bind _sequenceplayer (`self.SequencePlayer`)
    (:`then`
      (`self.K2_DestroyActor` _sequenceplayer))
    (:`else`)))

(fn `NextDialogue`
  (params (Data :type "DataTableRowHandle Structure"))
  (bind (_datatable _rowname) (break `DataTableRowHandle` Data))
  (bind (_datatable_2 _rowname_2) (break `DataTableRowHandle` Data))
  (bind _currentsubtitlesdelay (`self.CurrentSubtitlesDelay`))
  (bind _sequenceplayer (`LevelSequenceActor.SequencePlayer` (`self.SequencePlayer`)))
  (`/Engine/EditorBlueprintResources/StandardMacros.IsValid` (`.DataTable` (break `DataTableRowHandle` Data))
    (:`Is Valid`
      (if (== (`.DataTable` (break `DataTableRowHandle` Data)) (`self.NPC_DataTable`))
        (bind _returnvalue (`|GetDataTableRow` _datatable_2 _rowname_2)
          (:`then`
            (`/Engine/EditorBlueprintResources/StandardMacros.IsValid` (`self.SequencePlayer`)
              (:`Is Valid`
                (bind (_sequence _nextrow _subtitles _subtitlesdelay) (break `/Game/3CTemplates/TPSAT/Blueprints/Core/Structures/ConversationData_NPC` _returnvalue))
                (`LevelSequenceActor.SetSequence` (`self.SequencePlayer`) _sequence))
              (:`Is Not Valid`
                (bind _outactor (`LevelSequencePlayer.CreateLevelSequencePlayer` _sequence))
                (set `self.SequencePlayer` _outactor)))
            (set `self.NextUp` _nextrow)
            (set `self.CurrentSubtitles` _subtitles)
            (set `self.CurrentSubtitlesDelay` _subtitlesdelay)
            (set `self.CurrentSubtitleIndex` 0)
            (`MovieSceneSequencePlayer.Play` _sequenceplayer)
            (add `MovieSceneSequencePlayer.OnFinished` _sequenceplayer (`|CreateDelegate` :!event `CarryOnConversation`))
            (if (`KismetArrayLibrary.Array_IsValidIndex` _currentsubtitlesdelay)
              (`KismetSystemLibrary.K2_SetTimer` null "ShowSubtitles" (+ (`|GetArrayItem` _currentsubtitlesdelay) 0.1))
              (else
                (`KismetSystemLibrary.K2_SetTimer` null "ShowSubtitles")))))
        (else
          (bind _returnvalue_2 (`|GetDataTableRow` _datatable _rowname)
            (:`then`
              (bind ((`LoopSequence_25_382DAE584975CA8AF4812D82BDD76E90` _loopsequence) (`Options_18_481DF1F2451A53C331CB72A83146D35E` _options)) (break `/Game/3CTemplates/TPSAT/Blueprints/Core/Structures/ConversationData_Player` _returnvalue_2))
              (`self.DialogueOptions` _options _loopsequence))))))
    (:`Is Not Valid`
      ;[1 1 1 1 16] Back to game, set conversation over to true so we can play a comment when talking to NPC again. If there's no comment, disable talk interaction by clearing the button text
      (`self.EndConversation`)
      (set `self.ConversationOver` true)
      (`/Engine/EditorBlueprintResources/StandardMacros.IsValid` (`self.AfterConversationComment`)
        (:`Is Not Valid`
          (`self.DisableTalkButton`))))))

(fn `PlayCommentSequence`
  (`/Engine/EditorBlueprintResources/StandardMacros.IsValid` (`self.AfterConversationComment`)
    (:`Is Valid`
      (bind _outactor (`LevelSequencePlayer.CreateLevelSequencePlayer` (`self.AfterConversationComment`)))
      (set `self.SequencePlayer` _outactor)
      (`MovieSceneSequencePlayer.Play` (`LevelSequenceActor.SequencePlayer` (`self.SequencePlayer`)))
      (set `/Game/3CTemplates/TPSAT/Blueprints/Core/BP_StoryAdv_GameController.HoldTrace` true (`self.GameControllerInstance`))
      (bind _hiddenwidgets (`/Game/3CTemplates/TPSAT/Blueprints/Core/BP_StoryAdv_FunctionLibrary.HideActiveWidgets`))
      (set `self.HiddenWidgets` _hiddenwidgets)
      (`SceneComponent.SetHiddenInGame` (`self.Character`) true true)
      (`self.SetActorHiddenInGame` (`GameplayStatics.GetPlayerPawn` 0) true)
      (`self.DisableInput` (`self.GameControllerInstance`) (`GameplayStatics.GetPlayerController` 0))
      (`self.DisableInput` (`GameplayStatics.GetPlayerPawn` 0) (`GameplayStatics.GetPlayerController` 0))
      (add `MovieSceneSequencePlayer.OnFinished` (`LevelSequenceActor.SequencePlayer` (`self.SequencePlayer`)) (`|CreateDelegate` :!event `EndConversation`))
      (`self.ShowSubtitles`))
    (:`Is Not Valid`
      (setmembers `/Game/3CTemplates/TPSAT/Blueprints/Core/Structures/BP_InteractionLabels` :`StructRef` (`self.InteractionButtons`) :`Bottom Button` ""))))

(fn `SelectOption`
  (params (Index :type Integer))
  (bind _sequenceplayer (`self.SequencePlayer`))
  (bind _currentsubtitlesdelay (`self.CurrentSubtitlesDelay`))
  (bind _sequenceplayer_2 (`LevelSequenceActor.SequencePlayer` _sequenceplayer))
  (bind ((`Sequence_22_481DF1F2451A53C331CB72A83146D35E` _sequence) (`Response_25_A38183C94B8976885B0EBAA2AAA807F8` _response) (`Subtitles_29_2F87CEF24D981460CEADFBA946B31600` _subtitles) (`SubtitlesDelay_32_59A8F6BE426533A201D0EBA8AD051415` _subtitlesdelay) (`ConsequenceScript_35_2E1BB9F44368B76D2B479290369FC847` _consequencescript)) (break `/Game/3CTemplates/TPSAT/Blueprints/Core/Structures/Conversation_PlayerOptions` (`|GetArrayItem` (`self.CurrentDialogueOptions`) Index)))
  (set `self.NextUp` _response)
  (`/Game/3CTemplates/TPSAT/UserInterface/WBP_DialogueOptions.Clear` (`self.DialogueWidget`))
  (`MovieSceneSequencePlayer.Stop` (`LevelSequenceActor.SequencePlayer` (`self.SequencePlayer`)))
  (`LevelSequenceActor.SetSequence` _sequenceplayer _sequence)
  (`MovieSceneSequencePlayer.Play` _sequenceplayer_2)
  (add `MovieSceneSequencePlayer.OnFinished` _sequenceplayer_2 (`|CreateDelegate` :!event `CarryOnConversation`))
  (set `self.CurrentSubtitles` _subtitles)
  (set `self.CurrentSubtitlesDelay` _subtitlesdelay)
  (set `self.CurrentSubtitleIndex` 0)
  (`|ExecutionSequence`
    (:`then_0`
      ;[0 0.7379 1] Spawn and run consequence script if there is one
      (if (`KismetSystemLibrary.IsValidClass` _consequencescript)
        (bind _returnvalue (`|SpawnActorFromClass` _consequencescript (`KismetMathLibrary.MakeTransform` (0.0 0.0 0.0)) "AlwaysSpawn" "OverrideRootScale" null null))
        (`/Game/3CTemplates/TPSAT/Blueprints/Core/BaseActors/BP_Base_ConsequenceScript.RunScript` _returnvalue)))
    (:`then_1`
      ;[0 0.7379 1] Show subtitles
      (if (`KismetArrayLibrary.Array_IsValidIndex` _currentsubtitlesdelay)
        (`KismetSystemLibrary.K2_SetTimer` null "ShowSubtitles" (+ (`|GetArrayItem` _currentsubtitlesdelay) 0.1))
        (else
          (`KismetSystemLibrary.K2_SetTimer` null "ShowSubtitles" 0.1))))))

(fn `ShowSubtitles`
  (bind _currentsubtitlesdelay (`self.CurrentSubtitlesDelay`))
  (bind _currentsubtitleindex (`self.CurrentSubtitleIndex`))
  (bind _output (`|GetArrayItem` (`self.CurrentSubtitles`) (`self.CurrentSubtitleIndex`)))
  (bind _returnvalue (`KismetMathLibrary.MapRangeUnclamped` (`KismetMathLibrary.Conv_IntToDouble` (`KismetStringLibrary.Len` (`KismetTextLibrary.Conv_TextToString` _output))) 0.0 50.0 1.0 3.5))
  (if (`Widget.IsVisible` (`/Game/3CTemplates/TPSAT/Blueprints/Core/BP_StoryAdv_GameController.SubtitlesWidget` (`self.GameControllerInstance`)))
    (`KismetSystemLibrary.K2_SetTimer` null "ShowSubtitles" 0.1) ; Wait until there are no other subtitles currently displayed
    (else
      (`/Game/3CTemplates/TPSAT/UserInterface/WBP_Subtitles.ShowSubtitles` (`/Game/3CTemplates/TPSAT/Blueprints/Core/BP_StoryAdv_GameController.SubtitlesWidget` (`self.GameControllerInstance`)) _output _returnvalue)
      (if (`KismetArrayLibrary.Array_IsValidIndex` (`self.CurrentSubtitles`) (+ (`self.CurrentSubtitleIndex`) 1))
        (if (`KismetArrayLibrary.Array_IsValidIndex` _currentsubtitlesdelay _currentsubtitleindex)
          (`KismetSystemLibrary.K2_SetTimer` null "ShowSubtitles" (+ (`|GetArrayItem` _currentsubtitlesdelay _currentsubtitleindex) _returnvalue))
          (else
            (`KismetSystemLibrary.K2_SetTimer` null "ShowSubtitles" _returnvalue)))
        (`/Engine/EditorBlueprintResources/StandardMacros.IncrementInt` (`self.CurrentSubtitleIndex`))))))

(fn `UserConstructionScript`
  (`parent.UserConstructionScript`))