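; BP_Base_Simple_Inspection_Object is a base actor for simple inspectable objects that respond to a top-button interaction.
; On interaction, it looks up its DialogueRow in a data table and, if the data is valid, plays the player dialogue waves with subtitles through the game controller.
; It then triggers a camera focus when UseCameraFocus is enabled, regardless of whether dialogue played.
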(event `self.TopButtonInteraction`
  (`|ExecutionSequence`
    (:`then_0`
      (bind (_dialogue_waves _subtitles _validdata) (`/Game/3CTemplates/TPSAT/Blueprints/Core/BP_StoryAdv_FunctionLibrary.GetDialogueDataFromTable` (`self.DialogueRow`)))
      (if _validdata
        (`/Game/3CTemplates/TPSAT/Blueprints/Core/BP_StoryAdv_GameController.PlayPlayerDialogue` (`self.GameControllerInstance`) _dialogue_waves _subtitles)))
    (:`then_1`
      (if (`self.UseCameraFocus`)
        (`self.CameraFocus`)))))

(fn `UserConstructionScript`
  (`parent.UserConstructionScript`))